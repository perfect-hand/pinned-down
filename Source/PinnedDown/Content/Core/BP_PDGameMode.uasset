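; BP_PDGameMode is the game mode for a card game, providing the setup that readies a player's cards for play.
; PrepareToPlay puts the Flagship card into the InPlay pile and fills the DrawDeck pile from the given deck.
; It then shuffles the draw deck and moves InitialHandSize cards into the Hand, addressing each pile by a data-asset class.
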(fn `PrepareToPlay`
  (params (Player :type "Controller Object Reference") (Flagship :type "CardGameCard Object Reference") (Deck :type "Array of CardGameCard Object Reference"))
  (`|ExecutionSequence`
    (:`then_0`
      (`self.AddCardToPlayerCardPile` (`local.Player`) "/Game/Data/CardPiles/DA_CardPile_InPlay.DA_CardPile_InPlay" (`local.Flagship`)))
    (:`then_1`
      (for _array_element (`local.Deck`)
        (`self.AddCardToPlayerCardPile` (`local.Player`) "/Game/Data/CardPiles/DA_CardPile_DrawDeck.DA_CardPile_DrawDeck" _array_element)))
    (:`then_2`
      (`self.ShufflePlayerCardPile` (`local.Player`) "/Game/Data/CardPiles/DA_CardPile_DrawDeck.DA_CardPile_DrawDeck"))
    (:`then_3`
      (for _ (range (`self.InitialHandSize`))
        (`self.MoveCardBetweenPlayerPiles` (`local.Player`) "/Game/Data/CardPiles/DA_CardPile_DrawDeck.DA_CardPile_DrawDeck" "/Game/Data/CardPiles/DA_CardPile_Hand.DA_CardPile_Hand")))))

(fn `UserConstructionScript`)